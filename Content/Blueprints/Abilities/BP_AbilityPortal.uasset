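; Portal ability actor Blueprint that handles the portal's Niagara visual effect.
; The setup event spawns the particle system at the mesh location with the actor's rotation, stores the component and sets a high spawn rate.
; The destruction event zeroes the spawn rate, waits for the Lifespan delay so existing particles can fade, then destroys the component.
; Neither event is called within this graph.
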(event EventBeginPlay)

(event Collision|EventActorBeginOverlap
  (params (OtherActor :type Actor%20Object%20Reference)))

(event EventTick
  (params (DeltaSeconds :type Float%20%28single-precision%29)))

(event EventHandleNiagaraSetup
  (bind _returnvalue (Niagara|SpawnSystematLocation (Variables|Default|GetPortalParticleSystem) (Transformation|GetWorldLocation (Variables|Character|GetMesh)) (Transformation|GetActorRotation)))
  (bind _output_get (Variables|Default|SetNiagaraComp _returnvalue))
  (Effects|Components|ParticleSystem|SetFloatParameter _output_get "User.SpawnRate" 3e+04))

(event EventHandleNiagaraDestruction
  (Effects|Components|ParticleSystem|SetFloatParameter (Variables|Default|GetNiagaraComp) "User.SpawnRate" 0.0)
  (Utilities|FlowControl|Delay (Variables|Default|GetLifespan))
  (Components|DestroyComponent (Variables|Default|GetNiagaraComp)))

(fn ConstructionScript)